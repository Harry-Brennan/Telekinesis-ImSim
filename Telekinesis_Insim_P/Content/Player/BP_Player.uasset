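; Player character with first-person-style movement, timeline-blended crouch and sprint, and telekinetic lift and throw of physics bodies.
; Lift box-traces from the camera, then a looping timer applies mass-dependent forces toward an offset hold point.
; Charged throw launches the held object and starts a lift cooldown, or pushes sphere-traced bodies when empty-handed.
; Looping timers drive camera tilt, vertical-velocity bob and speed-based FOV; debug keys control a colour-isolation post-process material.
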(event Custom|Reset%20Throw%20Charge
  ;[0 0 0 1 194] TELEKINESIS
  (Utilities|FlowControl|DoOnce false) ; enters at Reset
)

(event Input|EnhancedActionEvents|EnhancedInputActionIA_Move
  (params (ActionValue :type Vector%202D%20Structure) (ElapsedSeconds :type Float%20%28double-precision%29) (TriggeredSeconds :type Float%20%28double-precision%29) (InputAction :type Input%20Action%20Object%20Reference :default "/Game/Player/Input/Actions/IA_Move.IA_Move"))
  (bind (_x _y) (Math|Vector2D|BreakVector2D ActionValue))
  ;[0 0 0] Basic movement and look
  (Pawn|Input|AddMovementInput (Transformation|GetActorRightVector) _x false)
  (Pawn|Input|AddMovementInput (Transformation|GetActorForwardVector) _y false)
  (Variables|Looking|SetCamera%20Movement%20Yaw (+ (Variables|Looking|GetCamera%20Movement%20Yaw) _x)))

(event Input|EnhancedActionEvents|EnhancedInputActionIA_Jump
  (params (ActionValue :type Boolean) (ElapsedSeconds :type Float%20%28double-precision%29) (TriggeredSeconds :type Float%20%28double-precision%29) (InputAction :type Input%20Action%20Object%20Reference :default "/Game/Player/Input/Actions/IA_Jump.IA_Jump"))
  ;[0 0 0] Basic movement and look
  (:Triggered
    (Character|Jump))
  (:Completed
    (Character|StopJumping)))

(event Input|EnhancedActionEvents|EnhancedInputActionIA_Look
  (params (ActionValue :type Vector%202D%20Structure) (ElapsedSeconds :type Float%20%28double-precision%29) (TriggeredSeconds :type Float%20%28double-precision%29) (InputAction :type Input%20Action%20Object%20Reference :default "/Game/Player/Input/Actions/IA_Look.IA_Look"))
  (bind _look_sens (Variables|Looking|GetLook%20Sens))
  (bind _returnvalue (* ActionValue _look_sens))
  (bind (_x _y) (Math|Vector2D|BreakVector2D _returnvalue))
  ;[0 0 0] Basic movement and look
  (Variables|Looking|SetCamera%20Movement%20Yaw (+ (Variables|Looking|GetCamera%20Movement%20Yaw) (/ _x 2.0)))
  (Pawn|Input|AddControllerYawInput _x)
  (Pawn|Input|AddControllerPitchInput _y))

(event Input|EnhancedActionEvents|EnhancedInputActionIA_Lift
  (params (ActionValue :type Boolean) (ElapsedSeconds :type Float%20%28double-precision%29) (TriggeredSeconds :type Float%20%28double-precision%29) (InputAction :type Input%20Action%20Object%20Reference :default "/Game/Player/Input/Actions/IA_Lift.IA_Lift"))
  (bind _camera (Variables|Default|GetCamera))
  (bind _returnvalue (Transformation|GetWorldLocation _camera))
  ;[0 0 0 1 194] TELEKINESIS
  (:Triggered
    (if (not (Variables|Telekinesis|GetLift%20Cooldown%20Active))
      (if (not (Variables|Telekinesis|GetLifting%20Obj))
        (bind (_outhit _returnvalue_2) (Class|KismetSystemLibrary|BoxTraceSingleforObjects _returnvalue (+ _returnvalue (* (Math|Vector|GetForwardVector _camera) 7.5e+02)) "32.000000,32.000000,32.000000" (Transformation|GetWorldRotation _camera) (Utilities|Array|MakeArray "ObjectTypeQuery4") false 0 "ForOneFrame" true))
        (if _returnvalue_2
          (Development|PrintString (Utilities|String|Append "LIFTING OBJECT: " (Utilities|GetDisplayName (.HitComponent (Collision|BreakHitResult _outhit)))))
          (Variables|Telekinesis|SetLifting%20Obj true)
          (Variables|Telekinesis|SetComponent%20Lifting (.HitComponent (Collision|BreakHitResult _outhit)))
          (bind _returnvalue_3 (Utilities|Time|SetTimerbyFunctionName 0 "Lift Obj Loop" 0.001 true))
          (Variables|Telekinesis|SetLift%20Obj%20Loop%20Timer _returnvalue_3)
          (else
            (Variables|Telekinesis|SetComponent%20Lifting 0))))))
  (:Completed
    (Development|PrintString "Completed")
    (Utilities|Time|ClearandInvalidateTimerbyHandle (Variables|Telekinesis|GetLift%20Obj%20Loop%20Timer))
    (Variables|Telekinesis|SetLifting%20Obj false)))

(event Input|EnhancedActionEvents|EnhancedInputActionIA_Throw
  (params (ActionValue :type Boolean) (ElapsedSeconds :type Float%20%28double-precision%29) (TriggeredSeconds :type Float%20%28double-precision%29) (InputAction :type Input%20Action%20Object%20Reference :default "/Game/Player/Input/Actions/IA_Throw.IA_Throw"))
  (bind _returnvalue (Transformation|GetActorLocation))
  ;[0 0 0 1 194] TELEKINESIS
  (:Ongoing
    (Utilities|FlowControl|Sequence
      (:then_0
        (Utilities|FlowControl|DoOnce false
          (:Completed
            (Variables|Telekinesis|SetThrow%20Charge 0.0))))
      (:then_1
        (bind _output_get (Variables|Telekinesis|SetThrow%20Charge (Math|Float|Clamp(Float) (+ (Variables|Telekinesis|GetThrow%20Charge) 0.01))))
        (if (== _output_get 1.0)
          (if (Variables|Telekinesis|GetLifting%20Obj) :!label _label
            (Variables|Telekinesis|SetLifting%20Obj false)
            (Utilities|Time|ClearandInvalidateTimerbyHandle (Variables|Telekinesis|GetLift%20Obj%20Loop%20Timer))
            (Utilities|Time|SetTimerbyFunctionName 0 "Lift Cooldown" 3.0)
            (Variables|Telekinesis|SetLift%20Cooldown%20Active true)
            (Physics|AddImpulse (Variables|Telekinesis|GetComponent%20Lifting) (* (Math|Vector|GetForwardVector (Variables|Default|GetCamera)) (Math|Float|MapRangeClamped (Variables|Telekinesis|GetThrow%20Charge) 0.0 1.0 0.0 7.5e+03)) "None" false)
            (Variables|Telekinesis|SetComponent%20Lifting 0)
            (else
              (bind (_outhits _returnvalue_2) (Collision|MultiSphereTraceForObjects _returnvalue (+ _returnvalue (* (Math|Vector|GetForwardVector (Variables|Default|GetCamera)) 7.5e+02)) 128.0 (Utilities|Array|MakeArray "ObjectTypeQuery4") false 0 "ForDuration"))
              (if _returnvalue_2
                (for _array_element _outhits
                  (Physics|AddImpulse (.HitComponent (Collision|BreakHitResult _array_element)) (* (Math|Vector|GetForwardVector (Variables|Default|GetCamera)) (* (Math|Float|MapRangeClamped (Variables|Telekinesis|GetThrow%20Charge) 0.0 1.0 0.0 7.5e+03) (Math|Float|MapRangeClamped (Physics|GetMass (.HitComponent (Collision|BreakHitResult _array_element))) 0.0 1e+02 1.0 3.0))) "None" false)))))
          (CallFunction|ResetThrowCharge)))))
  (:Completed
    (goto _label)))

(event Input|EnhancedActionEvents|EnhancedInputActionIA_Crouch
  (params (ActionValue :type Boolean) (ElapsedSeconds :type Float%20%28double-precision%29) (TriggeredSeconds :type Float%20%28double-precision%29) (InputAction :type Input%20Action%20Object%20Reference :default "/Game/Player/Input/Actions/IA_Crouch.IA_Crouch"))
  (bind _returnvalue (/ 1.0 0.25))
  (:Triggered
    (Components|Timeline|SetPlayRate (Variables|Default|GetCrouch%20Timeline) _returnvalue)
    (bind (_direction _alpha) (Timeline|Crouch%20Timeline Play)
      (:Update
        (Variables|/Script/Engine.CharacterMovementComponent|SetMaxWalkSpeed (Variables|Character|GetCharacterMovement) (Math|Float|Lerp (Variables|Movement|GetWalk%20Speed) (Variables|Movement|GetCrouch%20Speed) _alpha))
        (Components|Capsule|SetCapsuleHalfHeight (Variables|Collision|GetCapsuleComponent) (Math|Float|Lerp 88.0 44.0 _alpha) true))
      (:Finished
        (Variables|Movement|SetCrouching (Utilities|Enum|Equal(Enum) _direction "Forward")))))
  (:Completed
    (Components|Timeline|SetPlayRate (Variables|Default|GetCrouch%20Timeline) _returnvalue)
    (Timeline|Crouch%20Timeline Reverse)))

(event Input|EnhancedActionEvents|EnhancedInputActionIA_Sprint
  (params (ActionValue :type Boolean) (ElapsedSeconds :type Float%20%28double-precision%29) (TriggeredSeconds :type Float%20%28double-precision%29) (InputAction :type Input%20Action%20Object%20Reference :default "/Game/Player/Input/Actions/IA_Sprint.IA_Sprint"))
  (bind _returnvalue (/ 1.0 0.25))
  (:Triggered
    (Components|Timeline|SetPlayRate (Variables|Default|GetCrouch%20Timeline) _returnvalue)
    (bind (_direction _alpha) (Timeline|Sprint%20Timeline Play)
      (:Update
        (Variables|/Script/Engine.CharacterMovementComponent|SetMaxWalkSpeed (Variables|Character|GetCharacterMovement) (Math|Float|Lerp (Variables|Movement|GetWalk%20Speed) (Variables|Movement|GetSprint%20Speed) _alpha)))
      (:Finished
        (Variables|Movement|SetSprinting (Utilities|Enum|Equal(Enum) _direction "Forward")))))
  (:Completed
    (Components|Timeline|SetPlayRate (Variables|Default|GetCrouch%20Timeline) _returnvalue)
    (Timeline|Sprint%20Timeline Reverse)))

(event EventBeginPlay
  (Utilities|Time|SetTimerbyFunctionName 0 "Camera Tilt" 0.01 true)
  (Utilities|Time|SetTimerbyFunctionName 0 "Camera Land Jiggle" 0.01 true)
  (Utilities|Time|SetTimerbyFunctionName 0 "Camera FOV Movement" 0.01 true))

(event Input|KeyboardEvents|DebugKey1
  (params (Key :type Key%20Structure :default "None") (ActionValue :type Input%20Action%20Value%20Structure))
  (:Pressed
    (Rendering|Material|SetVectorParameterValue (Variables|PostProcess|GetSingle%20Colour%20PP) "Colour to isolate" "(R=1.000000,G=0.000000,B=0.000000,A=1.000000)" :!class /Script/Engine.MaterialInstanceDynamic)))

(event Input|KeyboardEvents|DebugKey3
  (params (Key :type Key%20Structure :default "None") (ActionValue :type Input%20Action%20Value%20Structure))
  (:Pressed
    (Rendering|Material|SetVectorParameterValue (Variables|PostProcess|GetSingle%20Colour%20PP) "Colour to isolate" "(R=0.000000,G=1.000000,B=0.000000,A=1.000000)" :!class /Script/Engine.MaterialInstanceDynamic)))

(event Input|KeyboardEvents|DebugKey2
  (params (Key :type Key%20Structure :default "None") (ActionValue :type Input%20Action%20Value%20Structure))
  (:Pressed
    (Rendering|Material|SetVectorParameterValue (Variables|PostProcess|GetSingle%20Colour%20PP) "Colour to isolate" "(R=0.000000,G=0.000000,B=1.000000,A=1.000000)" :!class /Script/Engine.MaterialInstanceDynamic)))

(event Input|KeyboardEvents|DebugKey0
  (params (Key :type Key%20Structure :default "None") (ActionValue :type Input%20Action%20Value%20Structure))
  (:Pressed
    (bind _returnvalue (Rendering|Material|CreateDynamicMaterialInstance "/Game/M_Colour_Single_PP.M_Colour_Single_PP" "None" "None" :!class /Script/Engine.KismetMaterialLibrary))
    (bind _output_get (Variables|PostProcess|SetSingle%20Colour%20PP _returnvalue))
    (Utilities|Array|AppendArray (Utilities|Struct|BreakWeightedBlendables (Utilities|Struct|BreakPostProcessSettings (Variables|/Script/Engine.CameraComponent|GetPostProcessSettings (Variables|Default|GetCamera)))) (Utilities|Array|MakeArray (Utilities|Struct|MakeWeightedBlendable 1.0 _output_get)))
    (bind _structout (Utilities|Struct|SetmembersinPostProcessSettings (Variables|/Script/Engine.CameraComponent|GetPostProcessSettings (Variables|Default|GetCamera)) (Utilities|Struct|MakeWeightedBlendables (Utilities|Struct|BreakWeightedBlendables (Utilities|Struct|BreakPostProcessSettings (Variables|/Script/Engine.CameraComponent|GetPostProcessSettings (Variables|Default|GetCamera)))))))
    (Variables|/Script/Engine.CameraComponent|SetPostProcessSettings (Variables|Default|GetCamera) _structout)))

(fn ConstructionScript)

(fn CameraTilt
  (bind _springarm (Variables|Default|GetSpringArm))
  (bind _relativerotation (Variables|/Script/Engine.SceneComponent|GetRelativeRotation _springarm))
  (Transformation|SetRelativeRotation _springarm (Math|Rotator|MakeRotator (Math|Interpolation|FInterpTo (.roll _relativerotation) (Math|Float|MapRangeClamped (Variables|Looking|GetCamera%20Movement%20Yaw) -1.0 1.0 -5.0 5.0) (Utilities|Time|GetWorldDeltaSeconds) 3.0) (.pitch _relativerotation) (.yaw _relativerotation)) false false)
  (Variables|Looking|SetCamera%20Movement%20Yaw (Math|Interpolation|FInterpTo (Variables|Looking|GetCamera%20Movement%20Yaw) 0.0 (Utilities|Time|GetWorldDeltaSeconds) 25.0)))

(fn CameraLandJiggle
  (Transformation|SetRelativeLocation (Variables|Default|GetSpringArm) (Math|Vector|MakeVector 0.0 0.0 (Math|Interpolation|FInterpTo (.z (Variables|/Script/Engine.SceneComponent|GetRelativeLocation (Variables|Default|GetSpringArm))) (Math|Float|MapRangeClamped (.z (Variables|/Script/Engine.MovementComponent|GetVelocity (Variables|Character|GetCharacterMovement))) -1.5e+02 0.0 -2e+01 4e+01) (Utilities|Time|GetWorldDeltaSeconds) 2.0)) false false))

(fn CameraFOVMovement
  (bind _charactermovement (Variables|Character|GetCharacterMovement))
  (bind _velocity (Variables|/Script/Engine.MovementComponent|GetVelocity _charactermovement))
  (bind _returnvalue (Math|Vector|VectorLength _velocity))
  (Camera|SetFieldOfView (Variables|Default|GetCamera) (Math|Interpolation|FInterpTo (Variables|/Script/Engine.CameraComponent|GetFieldOfView (Variables|Default|GetCamera)) (Math|Float|MapRangeClamped (Math|Float|SelectFloat (* _returnvalue -1.0) _returnvalue (< _returnvalue 0.0)) 0.0 7.5e+02 9e+01 105.0) (Utilities|Time|GetWorldDeltaSeconds) 1.0)))

(fn LiftObjLoop
  (bind _returnvalue (Transformation|GetActorLocation))
  (bind _camera (Variables|Default|GetCamera))
  (bind _component_lifting (Variables|Telekinesis|GetComponent%20Lifting))
  (bind _component_lifting_2 (Variables|Telekinesis|GetComponent%20Lifting))
  (bind _component_lifting_3 (Variables|Telekinesis|GetComponent%20Lifting))
  (bind _returnvalue_2 (Transformation|GetWorldLocation _component_lifting))
  (bind _returnvalue_3 (Math|Vector|GetUpVector _camera))
  (bind _returnvalue_4 (Physics|GetMass _component_lifting_2))
  (bind _returnvalue_5 (Physics|GetMass _component_lifting_3))
  (bind _returnvalue_6 (Math|Vector|GetForwardVector _camera))
  (bind _returnvalue_7 (Math|Vector|GetRightVector _camera))
  (bind _returnvalue_8 (Math|Float|MapRangeClamped _returnvalue_4 1.0 1e+02 0.05 1.0))
  (bind _returnvalue_9 (Math|Float|MapRangeClamped _returnvalue_5 0.0 1e+02 1.0 0.0))
  (bind _returnvalue_10 (* _returnvalue_6 2.5e+02))
  (bind _returnvalue_11 (* _returnvalue_3 5e+01))
  (bind _returnvalue_12 (* _returnvalue_7 5e+01))
  (bind _returnvalue_13 (+ _returnvalue _returnvalue_10 _returnvalue_12 _returnvalue_11))
  (bind _returnvalue_14 (Math|Rotator|FindLookatRotation _returnvalue_2 _returnvalue_13))
  (bind _returnvalue_15 (Math|Vector|Distance(Vector) _returnvalue_2 _returnvalue_13))
  (bind _returnvalue_16 (Math|Vector|GetForwardVector _returnvalue_14))
  (Rendering|Debug|DrawDebugBox :Center _returnvalue_13 :Extent "4.000000,4.000000,4.000000" :Duration 0.01 :Thickness 1.0)
  (Collision|LineTraceByChannel _returnvalue_2 (+ (* _returnvalue_16 5e+02) _returnvalue_2) "TraceTypeQuery1" false 0 "ForOneFrame")
  (Development|PrintString (Utilities|String|ToString(Float) _returnvalue_8))
  (Physics|AddForce (Variables|Telekinesis|GetComponent%20Lifting) (Math|Vector|SelectVector (* (* (- (* _returnvalue_16 (/ _returnvalue_15 _returnvalue_8)) (Transformation|GetComponentVelocity (Variables|Telekinesis|GetComponent%20Lifting))) (Physics|GetMass (Variables|Telekinesis|GetComponent%20Lifting))) _returnvalue_9) (* _returnvalue_16 (* (Math|Float|MapRangeUnclamped _returnvalue_15 0.0 2.5e+02 0.0 1.0) (Math|Float|MapRangeClamped (Physics|GetMass (Variables|Telekinesis|GetComponent%20Lifting)) 0.0 1e+02 2.5e+02 5e+03))) (> _returnvalue_9 0.75)) "None" false))

(fn LiftCooldown
  (Variables|Telekinesis|SetLift%20Cooldown%20Active false))