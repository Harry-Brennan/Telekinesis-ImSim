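; PC_Player is a player controller that registers the default input mapping and toggles the ability menu.
; BeginPlay adds IMC_Default to the Enhanced Input subsystem.
; IA_Ability_Menu removes the menu if it is in the viewport, restoring game-only input and hiding the cursor.
; Otherwise it creates a fresh WBP_Ability_Menu on each opening, switches to UI-only input focused on it, and shows the cursor.
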(event `self.ReceiveBeginPlay`
  (bind _returnvalue (subsystem `EnhancedInputLocalPlayerSubsystem`))
  (`/Engine/EditorBlueprintResources/StandardMacros.IsValid` _returnvalue
    (:`Is Valid`
      (`EnhancedInputSubsystemInterface.AddMappingContext` _returnvalue "/Game/Player/Input/IMC_Default.IMC_Default" 0 (struct)))))

(event `EnhancedInput|/Game/Player/Input/Actions/IA_Ability_Menu`
  (params (ActionValue :type Boolean) (ElapsedSeconds :type "Float (double-precision)") (TriggeredSeconds :type "Float (double-precision)") (InputAction :type "InputAction Object Reference" :default "/Game/Player/Input/Actions/IA_Ability_Menu.IA_Ability_Menu"))
  (bind _ability_menu (`self.Ability Menu`))
  (:`Triggered`
    (`/Engine/EditorBlueprintResources/StandardMacros.IsValid` _ability_menu
      (:`Is Valid`
        (if (`Widget.IsInViewport` _ability_menu)
          (`Widget.RemoveFromParent` (`self.Ability Menu`))
          (`WidgetBlueprintLibrary.SetInputMode_GameOnly` self)
          (set `self.bShowMouseCursor` false)
          (else
            (bind _returnvalue (`|CreateWidget` "/Game/UI/RadialMenu/WBP_Ability_Menu.WBP_Ability_Menu_C" :!label _label))
            (bind _output_get (set `self.Ability Menu` _returnvalue))
            (`UserWidget.AddToViewport` _output_get 0)
            (`WidgetBlueprintLibrary.SetInputMode_UIOnlyEx` self _output_get)
            (set `self.bShowMouseCursor` true))))
      (:`Is Not Valid`
        (goto _label)))))

(fn `UserConstructionScript`)